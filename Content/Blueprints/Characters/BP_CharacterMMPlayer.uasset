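; BP_CharacterMMPlayer is the player character, handling movement, look and selection in a mandala builder widget.
; On possession by BP_PlayerControlerMM it adds the default and mandala UI Enhanced Input mapping contexts.
; The list-selection input steps a wrapping index over the shape data and passes it to the externally supplied widget, though backward steps offset by TestArray's length.
; The BeginPlay timer event and IA_SelectList are empty.
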(event `SetBuilderWidget`
  (params (NewParam :type "/Game/UI/WBP_WidgetMandalaBuilder Object Reference"))
  (set `self.WidgetMandalaBuilder` NewParam))

(event `self.ReceiveBeginPlay`
  (`KismetSystemLibrary.K2_SetTimerDelegate` (delegate `CustomEvent`)))

(event `CustomEvent`)

(event `EnhancedInput|/Game/FirstPerson/Input/Actions/IA_Move`
  (params (ActionValue :type "Vector2D Structure") (ElapsedSeconds :type "Float (double-precision)") (TriggeredSeconds :type "Float (double-precision)") (InputAction :type "InputAction Object Reference" :default "/Game/FirstPerson/Input/Actions/IA_Move.IA_Move"))
  (:`Triggered`
    (`self.AddMovementInput` (`self.GetActorRightVector`) ActionValue_X)
    (`self.AddMovementInput` (`self.GetActorForwardVector`) ActionValue_Y)))

(event `EnhancedInput|/Game/FirstPerson/Input/Actions/IA_Look`
  (params (ActionValue :type "Vector2D Structure") (ElapsedSeconds :type "Float (double-precision)") (TriggeredSeconds :type "Float (double-precision)") (InputAction :type "InputAction Object Reference" :default "/Game/FirstPerson/Input/Actions/IA_Look.IA_Look"))
  (:`Triggered`
    (`self.AddControllerYawInput` ActionValue_X)
    (`self.AddControllerPitchInput` ActionValue_Y)))

(event `self.ReceivePossessed`
  (params (NewController :type "Controller Object Reference"))
  (bind _asbp_player_controler_mm (cast `/Game/Blueprints/Core/BP_PlayerControlerMM` NewController))
  (bind _returnvalue (pcsubsystem `EnhancedInputLocalPlayerSubsystem` _asbp_player_controler_mm))
  (`EnhancedInputSubsystemInterface.AddMappingContext` _returnvalue "/Game/FirstPerson/Input/IMC_Default.IMC_Default" 0 (struct))
  (`EnhancedInputSubsystemInterface.AddMappingContext` _returnvalue "/Game/Input/Mapping/IMC_MandalaUI.IMC_MandalaUI" 0 (struct)))

(event `EnhancedInput|/Game/Input/InputActions/IA_SelectListElement`
  (params (ActionValue :type "Float (double-precision)") (ElapsedSeconds :type "Float (double-precision)") (TriggeredSeconds :type "Float (double-precision)") (InputAction :type "InputAction Object Reference" :default "/Game/Input/InputActions/IA_SelectListElement.IA_SelectListElement"))
  (:`Triggered`
    (set `self.ActionValueSelectElement` ActionValue)
    (if (> (`self.ActionValueSelectElement`) 0.0)
      (bind _output_get (set `self.IndexTest` (mod (`KismetMathLibrary.FTrunc` (+ (`self.ActionValueSelectElement`) (`self.IndexTest`))) (`KismetArrayLibrary.Array_Length` (`WidgetMandalaBuilder.ShapeDataArray` (`self.WidgetMandalaBuilder`))))))
      (`/Game/UI/WBP_WidgetMandalaBuilder.SelectListInex` (`self.WidgetMandalaBuilder`) _output_get)
      (else
        (bind _output_get_2 (set `self.IndexTest` (mod (`KismetMathLibrary.FTrunc` (+ (`self.ActionValueSelectElement`) (`self.IndexTest`) (`KismetArrayLibrary.Array_Length` (`self.TestArray`)))) (`KismetArrayLibrary.Array_Length` (`WidgetMandalaBuilder.ShapeDataArray` (`self.WidgetMandalaBuilder`))))))
        (`/Game/UI/WBP_WidgetMandalaBuilder.SelectListInex` (`self.WidgetMandalaBuilder`) _output_get_2)))))

(event `EnhancedInput|/Game/Input/InputActions/IA_SelectList`
  (params (ActionValue :type "Float (double-precision)") (ElapsedSeconds :type "Float (double-precision)") (TriggeredSeconds :type "Float (double-precision)") (InputAction :type "InputAction Object Reference" :default "/Game/Input/InputActions/IA_SelectList.IA_SelectList")))

(fn `UserConstructionScript`)